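; BP_Platform_TwoBehaviors is a placeable moving platform that starts moving when something overlaps its CollisionArea.
; The LoopOption flag selects between two timelines, one for looping movement and one for on-demand movement.
; Either timeline drives a lerp between StartPosition and EndPosition that sets the PlatformMesh relative location without sweep.
; The overlap does not filter by actor, and no end-overlap handling stops or reverses the movement.
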(event OnComponentBeginOverlap(CollisionArea)
  (params (OverlappedComponent :type Primitive%20Component%20Object%20Reference) (OtherActor :type Actor%20Object%20Reference) (OtherComp :type Primitive%20Component%20Object%20Reference) (OtherBodyIndex :type Integer) (bFromSweep :type Boolean) (SweepResult :type Hit%20Result%20Structure%20%28by%20ref%29))
  ;[1 1 1] Platform Movement Mechanics Implementation
  (if (Variables|Default|GetbLoopOption)
    (bind _platformdirectionup (Timeline|PlatformMovementLoop Play)
      (:Update
        (Transformation|SetRelativeLocation (Variables|Default|GetPlatformMesh) (Math|Vector|Lerp(Vector) (Variables|Default|GetStartPosition) (Variables|Default|GetEndPosition) _platformdirectionup) false false)))
    (else
      (bind _platformdirection (Timeline|PlatformMoveOnDemand Play)
        (:Update
          (Transformation|SetRelativeLocation (Variables|Default|GetPlatformMesh) (Math|Vector|Lerp(Vector) (Variables|Default|GetStartPosition) (Variables|Default|GetEndPosition) _platformdirection) false false))))))

(fn ConstructionScript)